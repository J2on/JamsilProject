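; BP_PlayerCamera is a player camera pawn with keyboard panning, screen-edge mouse scrolling and wheel zoom.
; MouseMovement compares the cursor's scaled viewport position to ViewportEdgeThreshold, using hard-coded correction factors, to set forward and right scroll scales.
; MoveForward and MoveRight add movement along the control yaw, with nonzero axis input overriding those edge scales.
; The mouse wheel adjusts the spring arm length within a clamped range.
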(event EventBeginPlay)

(event Collision|EventActorBeginOverlap
  (params (OtherActor :type Actor%20Object%20Reference)))

(event EventTick
  (params (DeltaSeconds :type Float%20%28single-precision%29)))

(event Input|AxisEvents|InputAxisMoveForward
  (params (AxisValue :type Float%20%28single-precision%29))
  ;[1 1 1] Camera movement
  (Pawn|Input|AddMovementInput (Math|Vector|GetForwardVector (Math|Rotator|MakeRotator 0.0 0.0 (.yaw (Pawn|GetControlRotation :!class /Script/Engine.Pawn)))) (Math|Float|SelectFloat AxisValue (Variables|Default|GetMouseForwardScale) (!= AxisValue 0.0)) false))

(event Input|AxisEvents|InputAxisMoveRight
  (params (AxisValue :type Float%20%28single-precision%29))
  ;[1 1 1] Camera movement
  (Pawn|Input|AddMovementInput (Math|Vector|GetRightVector (Math|Rotator|MakeRotator 0.0 0.0 (.yaw (Pawn|GetControlRotation :!class /Script/Engine.Pawn)))) (Math|Float|SelectFloat AxisValue (Variables|Default|GetMouseRightScale) (!= AxisValue 0.0)) false))

(event Input|AxisEvents|InputAxisMouseMovement
  (params (AxisValue :type Float%20%28single-precision%29))
  ;[1 1 1] Camera movement
  (bind _returnvalue (Class|WidgetLayoutLibrary|GetMousePositiononViewport))
  (Variables|Default|SetMouseRightScale (Math|Float|SelectFloat -1.0 (Math|Float|SelectFloat 1.0 0.0 (> (/ (.x _returnvalue) (* (.x (Viewport|GetViewportSize)) 2.158352)) (- 1.0 (Variables|Default|GetViewportEdgeThreshold)))) (< (/ (.x _returnvalue) (* (.x (Viewport|GetViewportSize)) 2.158352)) (Variables|Default|GetViewportEdgeThreshold))))
  (bind _returnvalue_2 (Class|WidgetLayoutLibrary|GetMousePositiononViewport))
  (Variables|Default|SetMouseForwardScale (Math|Float|SelectFloat 1.0 (Math|Float|SelectFloat -1.0 0.0 (> (/ (+ (.y _returnvalue_2) 0.54055) (* (.y (Viewport|GetViewportSize)) 2.157838)) (- 1.0 (Variables|Default|GetViewportEdgeThreshold)))) (< (/ (+ (.y _returnvalue_2) 0.54055) (* (.y (Viewport|GetViewportSize)) 2.157838)) (Variables|Default|GetViewportEdgeThreshold)))))

(event Input|MouseEvents|MouseWheelAxis
  (params (AxisValue :type Float%20%28single-precision%29))
  ;[1 1 1] Camera movement
  ;;[1 1 1] ZoomIn/ZoomOut
  (Variables|/Script/Engine.SpringArmComponent|SetTargetArmLength (Variables|Default|GetSpringArm) (Math|Float|Clamp(Float) (+ (* AxisValue -1e+03) (Variables|/Script/Engine.SpringArmComponent|GetTargetArmLength (Variables|Default|GetSpringArm))) 1e+04 3e+04)))

(fn ConstructionScript)